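; Player controller that shows a grid control menu and lets the player click grid actors in the world.
; On BeginPlay it creates the UMG_GridControll widget and adds it to the viewport.
; Tab toggles the mouse cursor, switching between Game and UI and Game Only input modes.
; Left click traces from the deprojected mouse position and passes any hit BP_GridActor to the widget's ControllBall.
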(event EventBeginPlay
  (bind _returnvalue (UserInterface|CreateWidget "/Game/Grid/UMG_GridControll.UMG_GridControll_C" self))
  (bind _output_get (Variables|Default|SetMenu _returnvalue))
  (UserInterface|Viewport|AddtoViewport _output_get 0))

(event EventTick
  (params (DeltaSeconds :type Float%20%28single-precision%29)))

(event Input|MouseEvents|LeftMouseButton
  (params (Key :type Key%20Structure :default "None"))
  (bind (_locationx _locationy) (Game|Player|GetMousePosition))
  (bind _self self)
  (bind (_worldposition _worlddirection) (Class|GameplayStatics|DeprojectScreentoWorld _self (Math|Vector2D|MakeVector2D _locationx _locationy)))
  (:Pressed
    (bind _outhit (Collision|LineTraceByChannel _worldposition (+ _worldposition (* _worlddirection 5e+03)) "TraceTypeQuery3" false 0 "None"))
    (if (.bBlockingHit (Collision|BreakHitResult _outhit))
      (bind _asbp_grid_actor (Utilities|Casting|CastToBP_GridActor (.HitActor (Collision|BreakHitResult _outhit))))
      (Default|ControllBall (Variables|Default|GetMenu) _asbp_grid_actor))))

(event Input|KeyboardEvents|Tab
  (params (Key :type Key%20Structure :default "None"))
  (bind _self self)
  (:Pressed
    (bind _output_get (Variables|Default|SetbShowMouseCursor (not (Variables|Default|GetbShowMouseCursor))))
    (if _output_get
      (Input|SetInputModeGameandUI _self 0 "DoNotLock" true false)
      (else
        (Input|SetInputModeGameOnly _self false)))))

(fn ConstructionScript)