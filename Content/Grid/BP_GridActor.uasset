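; BP_GridActor is a sphere actor that queries a Manager for nearby actors and highlights them, apparently as a spatial-partition test.
; On BeginPlay it scales the sphere from the width of its Size bounds.
; When Controlled, each Tick deactivates the previous Near set, retrieves a new one using Size, activates it and draws a debug box.
; Activate and Deactivate switch the sphere's Color material parameter between yellow and white.
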(event EventBeginPlay
  (bind _size (Variables|Default|GetSize))
  (Transformation|SetWorldScale3D (Variables|Default|GetSphere) (Math|Conversions|ToVector(Float) (/ (/ (.x (- (.max _size) (.min _size))) 4.0) 1e+02))))

(event EventTick
  (params (DeltaSeconds :type Float%20%28single-precision%29))
  (bind _size (Variables|Default|GetSize))
  (bind _returnvalue (+ (.min _size) (.max _size)))
  (bind _returnvalue_2 (- (.max _size) (.min _size)))
  (if (Variables|Default|GetControlled)
    (Utilities|FlowControl|Sequence
      (:then_0
        (for _array_element (Variables|Default|GetNear)
          (Class|GridActor|Deactivate _array_element)))
      (:then_1
        (bind _returnvalue_3 (Class|GridDataManager|Retrieve (Variables|Default|GetManager) (Variables|Default|GetSize)))
        (bind _output_get (Variables|Default|SetNear _returnvalue_3))
        (for _array_element_2 _output_get
          (Class|GridActor|Activate _array_element_2)))
      (:then_2
        (Rendering|Debug|DrawDebugBox (Math|Vector|MakeVector (/ (.x _returnvalue) 2.0) (/ (.y _returnvalue) 2.0) 1e+02) (Math|Vector|MakeVector (/ (.x _returnvalue_2) 4.0) (/ (.y _returnvalue_2) 4.0) 0.0) "(R=1.000000,G=0.000000,B=0.008304,A=1.000000)" "0, 0, 0" 0.0 1e+01)))))

(event EventActivate
  (Rendering|Material|SetVectorParameterValueonMaterials (Variables|Default|GetSphere) "Color" "1.000000,0.730000,0.000000"))

(event EventDeactivate
  (Rendering|Material|SetVectorParameterValueonMaterials (Variables|Default|GetSphere) "Color" "1.000000,1.000000,1.000000"))

(fn ConstructionScript)